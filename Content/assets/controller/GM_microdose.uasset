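; GM_microdose is a game mode Blueprint that drives the app's UI screen flow.
; On BeginPlay it creates the start screen widget for player 0 and adds it to the viewport.
; Its SetWidget interface event swaps screens by removing the passed widget, creating the requested class, setting UI-only input focused on it and showing it.
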(event EventBeginPlay
  (bind _returnvalue (UserInterface|CreateWidget "/Game/assets/UI/login_signup/UI_start_screen.UI_start_screen_C" (Game|GetPlayerController 0)))
  (UserInterface|Viewport|AddtoViewport _returnvalue 0))

(event EventTick
  (params (DeltaSeconds :type Float%20%28single-precision%29)))

(event EventSetWidget
  (params (widget_class :type User%20Widget%20Class%20Reference) (widget_object :type User%20Widget%20Object%20Reference))
  (bind _returnvalue (Game|GetPlayerController 0))
  ;[1 1 1] interace function
  (Widget|RemovefromParent widget_object)
  (bind _returnvalue_2 (UserInterface|CreateWidget widget_class _returnvalue))
  (Input|SetInputModeUIOnly _returnvalue _returnvalue_2 "DoNotLock" false)
  (UserInterface|Viewport|AddtoViewport _returnvalue_2 0)
  (Development|PrintString "widget changed" true true "(R=0.202697,G=1.000000,B=0.000000,A=1.000000)"))

(fn ConstructionScript)